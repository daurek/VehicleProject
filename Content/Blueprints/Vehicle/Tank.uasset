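; Player-driven wheeled tank vehicle that drives, aims with the mouse cursor and fires projectiles.
; Axis inputs interpolate front-wheel steering, torque the rear four wheels and toggle nitro trails when moving forward; R teleports back to spawn.
; Each tick a cursor trace yaws the turret platform and, beyond a minimum distance, pitches the arrow and draws a debug aim line.
; Left click spawns a projectile at the shoot point.
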(event `self.ReceiveBeginPlay`
  (set `self.SpawnLocation` (`SceneComponent.K2_GetComponentLocation` (`self.SkeletalMesh`))))

(event `self.ReceiveTick`
  (params (DeltaSeconds :type "Float (single-precision)"))
  (bind _arrow (`self.Arrow`))
  (bind _platform (`self.Platform`))
  (bind (_returnvalue_roll _returnvalue_pitch _returnvalue_yaw) (`KismetMathLibrary.BreakRotator` (`SceneComponent.K2_GetComponentRotation` _arrow)))
  (bind (_returnvalue_roll_2 _returnvalue_pitch_2) (`KismetMathLibrary.BreakRotator` (`SceneComponent.K2_GetComponentRotation` _platform)))
  (bind _returnvalue (`SceneComponent.K2_GetComponentLocation` _platform))
  (bind (_worldlocation _worlddirection) (`PlayerController.DeprojectMousePositionToWorld` (`GameplayStatics.GetPlayerController` 0)))
  (bind (_outhit _returnvalue_2) (`KismetSystemLibrary.LineTraceSingle` _worldlocation (+ _worldlocation (* _worlddirection 1000000)) "TraceTypeQuery2"))
  (if _returnvalue_2
    (set `self.LastLoc` (`.Location` (`GameplayStatics.BreakHitResult` _outhit)))
    (`SceneComponent.K2_SetWorldRotation` _platform (`KismetMathLibrary.MakeRotator` (.roll (`KismetMathLibrary.FindLookAtRotation` _returnvalue (`.Location` (`GameplayStatics.BreakHitResult` _outhit)))) _returnvalue_pitch_2 (.yaw (`KismetMathLibrary.FindLookAtRotation` _returnvalue (`.Location` (`GameplayStatics.BreakHitResult` _outhit))))) false false)
    (if (>= (`KismetMathLibrary.VSize` (- _returnvalue (`.Location` (`GameplayStatics.BreakHitResult` _outhit)))) 500.0)
      (`SceneComponent.K2_SetWorldRotation` _arrow (`KismetMathLibrary.MakeRotator` _returnvalue_roll (.pitch (`KismetMathLibrary.FindLookAtRotation` _returnvalue (`.Location` (`GameplayStatics.BreakHitResult` _outhit)))) _returnvalue_yaw) false false)
      (`KismetSystemLibrary.DrawDebugLine` (`SceneComponent.K2_GetComponentLocation` (`self.ShootPoint`)) (`self.LastLoc`) (struct :`R` 1.0 :`G` 0.073312 :`A` 1.0) 0.0 5.0))))

(event `InputAxis|Horizontal`
  (params (AxisValue :type "Float (single-precision)"))
  (bind _simplewheeledvehiclemovement (`self.SimpleWheeledVehicleMovement`))
  (bind _output_get (set `self.Steering` (`KismetMathLibrary.FInterpTo` (`self.Steering`) (* AxisValue 30.0) (`GameplayStatics.GetWorldDeltaSeconds`))))
  (`SimpleWheeledVehicleMovementComponent.SetSteerAngle` _simplewheeledvehiclemovement _output_get 0)
  (`SimpleWheeledVehicleMovementComponent.SetSteerAngle` _simplewheeledvehiclemovement _output_get 1))

(event `InputAxis|Vertical`
  (params (AxisValue :type "Float (single-precision)"))
  (bind _returnvalue (* AxisValue 400.0))
  (bind _nitro1 (`self.Nitro1`))
  (bind _nitro2 (`self.Nitro2`))
  (bind _simplewheeledvehiclemovement (`self.SimpleWheeledVehicleMovement`))
  (`|ExecutionSequence`
    (:`then_0`
      (if (> AxisValue 0.0)
        (`ActorComponent.Activate` _nitro1 false)
        (`ActorComponent.Activate` _nitro2 false)
        (else
          (`ActorComponent.Deactivate` _nitro1)
          (`ActorComponent.Deactivate` _nitro2))))
    (:`then_1`
      (`SimpleWheeledVehicleMovementComponent.SetDriveTorque` _simplewheeledvehiclemovement _returnvalue 2)
      (`SimpleWheeledVehicleMovementComponent.SetDriveTorque` _simplewheeledvehiclemovement _returnvalue 3)
      (`SimpleWheeledVehicleMovementComponent.SetDriveTorque` _simplewheeledvehiclemovement _returnvalue 4)
      (`SimpleWheeledVehicleMovementComponent.SetDriveTorque` _simplewheeledvehiclemovement _returnvalue 5))))

(event `Key|LeftMouseButton`
  (params (Key :type "Key Structure"))
  (bind (_returnvalue_location _returnvalue_rotation) (`KismetMathLibrary.BreakTransform` (`SceneComponent.K2_GetComponentToWorld` (`self.ShootPoint`))))
  (:`Pressed`
    (`|SpawnActorFromClass` "/Game/Blueprints/Projectile.Projectile_C" (`KismetMathLibrary.MakeTransform` _returnvalue_location _returnvalue_rotation) "Undefined" "OverrideRootScale" null null)))

(event `Key|R`
  (params (Key :type "Key Structure"))
  (:`Pressed`
    (`SceneComponent.K2_SetWorldLocation` (`self.SkeletalMesh`) (`self.SpawnLocation`) false true)))

(fn `UserConstructionScript`)