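; MyVehicle is a player-driven vehicle Blueprint with a speed boost.
; Horizontal and Vertical axis inputs feed steering and throttle into the VehicleMovement component.
; Pressing Left Shift multiplies the mesh's physics linear velocity once, guarded by IsBoostActivated; releasing it clears the flag and divides the current velocity by the same factor, rather than applying continuous force.
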(event `InputAxis|Horizontal`
  (params (AxisValue :type "Float (single-precision)"))
  (`WheeledVehicleMovementComponent.SetSteeringInput` (`self.VehicleMovement`) AxisValue))

(event `InputAxis|Vertical`
  (params (AxisValue :type "Float (single-precision)"))
  (`WheeledVehicleMovementComponent.SetThrottleInput` (`self.VehicleMovement`) AxisValue))

(event `Key|LeftShift`
  (params (Key :type "Key Structure"))
  (bind _mesh (`self.Mesh`))
  (bind _mesh_2 (`self.Mesh`))
  (:`Pressed`
    (if (not (`self.isBoostActivated`))
      (set `self.isBoostActivated` true)
      (bind _returnvalue (`PrimitiveComponent.GetPhysicsLinearVelocity` _mesh_2 "None"))
      (`PrimitiveComponent.SetPhysicsLinearVelocity` _mesh_2 (* _returnvalue 2.5) false "None")))
  (:`Released`
    (set `self.isBoostActivated` false)
    (bind _returnvalue_2 (`PrimitiveComponent.GetPhysicsLinearVelocity` _mesh "None"))
    (`PrimitiveComponent.SetPhysicsLinearVelocity` _mesh (/ _returnvalue_2 2.5) false "None")))

(fn `UserConstructionScript`)